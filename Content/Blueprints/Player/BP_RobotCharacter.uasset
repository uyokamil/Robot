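; Robot player character Blueprint that turns its mesh according to the direction of movement.
; Each Tick, it builds a rotator with MakeRotFromZ from the negated, normalized velocity and keeps only the yaw, zeroing pitch and roll.
; RInterpTo smooths the mesh's world rotation toward that yaw, and the construction script is empty.
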(event `self.ReceiveTick`
  (params (DeltaSeconds :type "Float (single-precision)"))
  (`SceneComponent.K2_SetWorldRotation` (`self.Mesh`) (`KismetMathLibrary.RInterpTo` (`SceneComponent.K2_GetComponentRotation` (`self.Mesh`)) (`KismetMathLibrary.MakeRotator` 0.0 0.0 (.yaw (`KismetMathLibrary.MakeRotFromZ` (* (`KismetMathLibrary.Normal` (`self.GetVelocity`)) -1.0)))) DeltaSeconds 30.0) false false))

(fn `UserConstructionScript`)